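; Player controller for Dungeon Runners that handles mouse-look, the HUD menu and the ability draft flow.
; Holding right mouse turns the pawn with controller yaw, hiding the cursor and pinning it each tick.
; A client event opens the HUD draft window with three abilities, and picks go through server events into the pawn's available abilities.
; Closing the draft readies the player in DraftGameMode, and another server event equips abilities to slots.
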(event Custom|ClientOpenDraftWindow
  (params (Ability1 :type Gameplay%20Ability%20Class%20Reference) (Ability2 :type Gameplay%20Ability%20Class%20Reference) (Ability3 :type Gameplay%20Ability%20Class%20Reference))
  (CallFunction|OpenDraftMenu Ability1 Ability2 Ability3))

(event Custom|ServerReadyAPlayer
  (bind _asdraft_game_mode (Utilities|Casting|CastToDraftGameMode (Game|GetGameMode)))
  (Default|ReadyAPlayer _asdraft_game_mode))

(event EventBeginPlay
  (Variables|/Script/Engine.Pawn|SetbUseControllerRotationYaw (Pawn|GetControlledPawn) false)
  (Variables|Default|SetbShowMouseCursor true)
  (Variables|Default|SetRMBDown false))

(event EventTick
  (params (DeltaSeconds :type Float%20%28single-precision%29))
  (if (Variables|Default|GetRMBDown)
    (Class|PlayerController|SetMouseLocation (Variables|Default|GetLastMouseX) (Variables|Default|GetLastMouseY))))

(event Input|ActionEvents|InputActionOpenMenu
  (params (Key :type Key%20Structure))
  (:Pressed
    (CallFunction|ToggleMenu)))

(event Input|MouseEvents|RightMouseButton
  (params (Key :type Key%20Structure))
  (bind (_locationx _locationy) (Game|Player|GetMousePosition))
  (bind _returnvalue (Pawn|GetControlledPawn))
  (:Pressed
    (Variables|/Script/Engine.Pawn|SetbUseControllerRotationYaw _returnvalue true)
    (Variables|Default|SetbShowMouseCursor false)
    (Variables|Default|SetRMBDown true)
    (Variables|Default|SetLastMouseX (Math|Float|Truncate _locationx))
    (Variables|Default|SetLastMouseY (Math|Float|Truncate _locationy)))
  (:Released
    (Variables|/Script/Engine.Pawn|SetbUseControllerRotationYaw _returnvalue false)
    (Variables|Default|SetbShowMouseCursor true)
    (Variables|Default|SetRMBDown false)))

(event Custom|ServerDraftAbility
  (params (Ability :type Gameplay%20Ability%20Class%20Reference))
  (CallFunction|DraftAbility Ability))

(event Custom|ServerEquipAbility
  (params (Character :type Dungeon%20Runners%20Character%20Object%20Reference) (Skill :type Gameplay%20Ability%20Class%20Reference) (Slot :type Integer))
  (Class|DungeonRunnersBPLib|EquipAbilitytoSlot Character Skill Slot))

(fn ConstructionScript)

(fn ToggleMenu
  (if (Variables|Default|GetMenuOpen)
    (CallFunction|CloseMenu)
    (else
      (CallFunction|OpenMenu))))

(fn OpenMenu
  (Variables|Default|SetMenuOpen true)
  (bind _asdungeon_runners_hud (Utilities|Casting|CastToDungeonRunnersHUD (HUD|GetHUD)))
  (Default|OpenMenu _asdungeon_runners_hud))

(fn CloseMenu
  (Variables|Default|SetMenuOpen false)
  (bind _asdungeon_runners_hud (Utilities|Casting|CastToDungeonRunnersHUD (HUD|GetHUD)))
  (Default|CloseMenu _asdungeon_runners_hud))

(fn DraftAbility
  (params (SkillToDraft :type Gameplay%20Ability%20Class%20Reference))
  (Development|PrintString (Utilities|String|Append "Drafting Skill: \"" (Utilities|GetClassDisplayName SkillToDraft) "\""))
  (bind _asplayer_character (Utilities|Casting|CastToPlayerCharacter (Pawn|GetControlledPawn)))
  (Utilities|Array|AddUnique (Variables|/Game/ThirdPersonCPP/Blueprints/PlayerCharacter.PlayerCharacter_C|GetAvailableAbilities _asplayer_character) SkillToDraft))

(fn OpenDraftMenu
  (params (Ability1 :type Gameplay%20Ability%20Class%20Reference) (Ability2 :type Gameplay%20Ability%20Class%20Reference) (Ability3 :type Gameplay%20Ability%20Class%20Reference))
  (bind _asdungeon_runners_hud (Utilities|Casting|CastToDungeonRunnersHUD (HUD|GetHUD)))
  (Default|InitDraftWindow (Variables|/Game/Blueprints/HUD/DungeonRunnersHUD.DungeonRunnersHUD_C|GetDraftWidget _asdungeon_runners_hud) Ability1 Ability2 Ability3)
  (Default|OpenDraftMenu _asdungeon_runners_hud))

(fn CloseDraftMenu
  (CallFunction|ServerReadyAPlayer)
  (bind _asdungeon_runners_hud (Utilities|Casting|CastToDungeonRunnersHUD (HUD|GetHUD)))
  (Default|CloseDraftMenu _asdungeon_runners_hud))

(fn TryDraftAbility
  (params (AbilityToDraft :type Gameplay%20Ability%20Class%20Reference))
  (CallFunction|ServerDraftAbility AbilityToDraft))