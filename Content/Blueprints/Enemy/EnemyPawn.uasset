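; EnemyPawn is an enemy character that feeds sighted players to its AI and keeps that AI in step with launches.
; PawnSensing passes each seen DungeonRunnersCharacter to the BaseAIController's threat map.
; Being launched stops the controller's movement, and landing calls AITick on the EnemyController.
; A PrintHealth helper prints a float attribute read from the Ability System.
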(event OnSeePawn(PawnSensing)
  (params (Pawn :type Pawn%20Object%20Reference))
  (bind _asdungeon_runners_character (Utilities|Casting|CastToDungeonRunnersCharacter Pawn))
  (bind _asbase_aicontroller (Utilities|Casting|CastToBaseAIController (AI|GetAIController self)))
  (Class|BaseAIController|TryAddCharactertoThreatMap _asbase_aicontroller _asdungeon_runners_character))

(event EventBeginPlay)

(event Collision|EventActorBeginOverlap
  (params (OtherActor :type Actor%20Object%20Reference)))

(event EventOnLanded
  (params (Hit :type Hit%20Result%20Structure%20%28by%20ref%29))
  (bind _self self)
  (bind _returnvalue (AI|GetAIController _self))
  (|CallParentFunction Hit)
  (Utilities|IsValid _returnvalue
    (:Is%20Valid
      (bind _asenemy_controller (Utilities|Casting|CastToEnemyController _returnvalue))
      (Default|AITick _asenemy_controller))))

(event EventOnLaunched
  (params (LaunchVelocity :type Vector :default "0, 0, 0") (bXYOverride :type Boolean) (bZOverride :type Boolean))
  (bind _self self)
  (bind _returnvalue (AI|GetAIController _self))
  (|CallParentFunction LaunchVelocity bXYOverride bZOverride)
  (Utilities|IsValid _returnvalue
    (:Is%20Valid
      (AI|Navigation|StopMovement _returnvalue))))

(event EventTick
  (params (DeltaSeconds :type Float%20%28single-precision%29)))

(fn ConstructionScript)

(fn PrintHealth
  (Development|PrintString (Utilities|String|ToString(Float) (.ReturnValue (Ability|Attribute|GetFloatAttributefromAbilitySystemComponent (Variables|Default|GetAbilitySystem) "(AttributeName=\"\",Attribute=None,AttributeOwner=None)")))))