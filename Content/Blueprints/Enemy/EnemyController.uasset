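; Enemy AI controller that chases a threat-based target and attacks it with a cleave ability.
; A looping one-second timer runs AITick, which calls FindTopThreat unless taunted, so a taunt holds the current target.
; It moves to and focuses on a valid target, then activates EnemyCleave through the pawn's Gameplay Ability System component once within attack range.
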(event Custom|AITick
  (bind _returnvalue (Pawn|GetControlledPawn))
  (bind _currenttarget (Variables|Default|GetCurrentTarget))
  (if (Variables|Default|GetbIsTaunted)
    _
    (else
      (Class|BaseAIController|FindTopThreat)))
  (Utilities|IsValid _currenttarget
    (:Is%20Valid
      (AI|Navigation|MovetoActor _currenttarget (* (Variables|Default|GetAttackRange) 0.6) true true)
      (AI|SetFocus _currenttarget)
      (if (<= (Transformation|GetDistanceTo _returnvalue _currenttarget) (Variables|Default|GetAttackRange))
        (bind _asdungeon_runners_character (Utilities|Casting|CastToDungeonRunnersCharacter _returnvalue))
        (Abilities|TryActivateAbilitybyClass (Ability|GetAbilitySystemComponent _asdungeon_runners_character) "/Game/Blueprints/Enemy/EnemyCleave.EnemyCleave_C" true)))))

(event EventBeginPlay
  (Utilities|Time|SetTimerbyEvent (delegate Custom|AITick) 1.0 true))

(fn ConstructionScript)