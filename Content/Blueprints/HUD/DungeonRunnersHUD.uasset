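; Dungeon Runners HUD that creates the main HUD widget plus hidden character and draft menus, with functions to open and close each menu.
; A looping timer scans for other DungeonRunnersCharacters and adds a unit frame for each new one.
; Global damage and heal events involving the owning pawn spawn color-coded scrolling combat text at the target's location.
; DrawHUD ticks the unit frames and repositions the floating texts every frame.
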(event Custom|OnEffectDamage
  (params (DamageAmount :type Float%20%28single-precision%29) (Source :type Dungeon%20Runners%20Character%20Object%20Reference) (Target :type Dungeon%20Runners%20Character%20Object%20Reference) (Crit :type Boolean))
  (CallFunction|OnEffectDamageHandler DamageAmount Source Target Crit))

(event Custom|OnEffectHeal
  (params (HealAmount :type Float%20%28single-precision%29) (Source :type Dungeon%20Runners%20Character%20Object%20Reference) (Target :type Dungeon%20Runners%20Character%20Object%20Reference) (Crit :type Boolean))
  (CallFunction|OnEffectHealDamageHandler HealAmount Source Target Crit))

(event EventBeginPlay
  (bind _returnvalue (Class|DungeonRunnersGameState|GetDungeonRunnersGameState))
  (bind _globaleventsystem (Variables|/Script/DungeonRunners.DungeonRunnersGameState|GetGlobalEventSystem _returnvalue))
  (CallFunction|AddCharacterMenu)
  (CallFunction|AddDraftMenu)
  (bind _returnvalue_2 (UserInterface|CreateWidget "/Game/Blueprints/HUD/DungeonRunnersHUDWidget.DungeonRunnersHUDWidget_C"))
  (bind _output_get (Variables|Default|SetHUDWidget _returnvalue_2))
  (bind _asdungeon_runners_character (Utilities|Casting|CastToDungeonRunnersCharacter (Pawn|GetControlledPawn (Game|Player|GetOwningPlayerController))))
  (Default|InitActionButtons _output_get _asdungeon_runners_character)
  (UserInterface|Viewport|AddtoViewport _output_get 0)
  (Utilities|Time|SetTimerbyFunctionName 0 "SearchActors" 0.5 true)
  (EventDispatchers|AssignOnEffectDamage _globaleventsystem (delegate Custom|OnEffectDamage))
  (EventDispatchers|AssignOnEffectHeal _globaleventsystem (delegate Custom|OnEffectHeal)))

(event EventDrawHUD
  (params (SizeX :type Integer) (SizeY :type Integer))
  (bind _values (Utilities|Map|Values (Variables|Default|GetUnitFrames)))
  (for _array_element _values
    (Default|WidgetTick _array_element))
  (for _array_element_2 (Variables|Default|GetScrollingTexts)
    (bind _asscrolling_combat_text_widget (Utilities|Casting|CastToScrollingCombatTextWidget _array_element_2))
    (Default|UpdatePosition _asscrolling_combat_text_widget)))

(fn ConstructionScript)

(fn SearchActors
  (bind _unitframes (Variables|Default|GetUnitFrames))
  (bind _outactors (Actor|GetAllActorsOfClass "/Script/DungeonRunners.DungeonRunnersCharacter"))
  (for _array_element _outactors
    (if (not (Utilities|Map|Contains _unitframes _array_element))
      (if (!= _array_element (Class|HUD|GetOwningPawn))
        (bind _returnvalue (UserInterface|CreateWidget "/Game/Blueprints/HUD/UnitFrameWidget.UnitFrameWidget_C" (Game|Player|GetOwningPlayerController)))
        (Default|CharacterFound _returnvalue _array_element)
        (UserInterface|Viewport|AddtoViewport _returnvalue 0)
        (Utilities|Map|Add _unitframes _array_element _returnvalue)))))

(fn OnEffectDamageHandler
  (params (DamageAmount :type Float%20%28single-precision%29) (Source :type Dungeon%20Runners%20Character%20Object%20Reference) (Target :type Dungeon%20Runners%20Character%20Object%20Reference) (Crit :type Boolean))
  (bind _returnvalue (Class|HUD|GetOwningPawn))
  (if (== Target _returnvalue)
    (CallFunction|MakeScrollingCombatWidget DamageAmount Target Crit (Utilities|Struct|MakeSlateColor "(R=1.000000,G=0.000000,B=0.000000,A=1.000000)"))
    (elif (== Source _returnvalue)
      (CallFunction|MakeScrollingCombatWidget DamageAmount Target Crit (Utilities|Struct|MakeSlateColor "(R=1.000000,G=1.000000,B=0.000000,A=1.000000)")))))

(fn OnEffectHealDamageHandler
  (params (HealAmount :type Float%20%28single-precision%29) (Source :type Dungeon%20Runners%20Character%20Object%20Reference) (Target :type Dungeon%20Runners%20Character%20Object%20Reference) (Crit :type Boolean))
  (bind _returnvalue (Class|HUD|GetOwningPawn))
  (if (== Source _returnvalue)
    (CallFunction|MakeScrollingCombatWidget HealAmount Target false (Utilities|Struct|MakeSlateColor "(R=0.000000,G=1.000000,B=0.000000,A=1.000000)") :!label _label)
    (elif (== Target _returnvalue)
      (goto _label))))

(fn MakeScrollingCombatWidget
  (params (Amount :type Float%20%28single-precision%29) (TargetActor :type Dungeon%20Runners%20Character%20Object%20Reference) (Crit :type Boolean) (TextColor :type Slate%20Color%20Structure))
  (bind _returnvalue (UserInterface|CreateWidget "/Game/Blueprints/HUD/ScrollingCombatTextWidget.ScrollingCombatTextWidget_C" (Game|Player|GetOwningPlayerController) Amount Crit (Transformation|GetActorLocation TargetActor) TextColor))
  (UserInterface|Viewport|AddtoViewport _returnvalue 0)
  (Utilities|Array|AddUnique (Variables|Default|GetScrollingTexts) _returnvalue))

(fn AddCharacterMenu
  (bind _returnvalue (UserInterface|CreateWidget "/Game/Blueprints/HUD/Menu.Menu_C"))
  (bind _output_get (Variables|Default|SetMenuWidget _returnvalue))
  (Widget|SetVisibility _output_get "Hidden")
  (UserInterface|Viewport|AddtoViewport _output_get 0))

(fn AddDraftMenu
  (bind _returnvalue (UserInterface|CreateWidget "/Game/Blueprints/HUD/DraftMenu.DraftMenu_C"))
  (bind _output_get (Variables|Default|SetDraftWidget _returnvalue))
  (Widget|SetVisibility _output_get "Hidden")
  (UserInterface|Viewport|AddtoViewport _output_get 0))

(fn CloseMenu
  (Widget|SetVisibility (Variables|Default|GetMenuWidget) "Hidden"))

(fn CloseDraftMenu
  (Widget|SetVisibility (Variables|Default|GetDraftWidget) "Hidden"))

(fn OpenMenu
  (bind _menuwidget (Variables|Default|GetMenuWidget))
  (Default|RefreshAbilityPanel _menuwidget)
  (Widget|SetVisibility _menuwidget "Visible"))

(fn OpenDraftMenu
  (Widget|SetVisibility (Variables|Default|GetDraftWidget) "Visible"))