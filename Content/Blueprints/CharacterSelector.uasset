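; CharacterSelector is an overlap-triggered actor that swaps a player's pawn for a selected character class.
; On authority, an overlapping DungeonRunnersCharacter triggers a spawn of SelectedClass at the Teleport location, and that character's controller possesses the new actor.
; The old pawn is then passed to the ClientCharacterSelect event, which destroys it.
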(event Custom|ClientCharacterSelect
  (params (OldPawn :type Dungeon%20Runners%20Character%20Object%20Reference))
  (Actor|DestroyActor OldPawn))

(event EventBeginPlay)

(event Collision|EventActorBeginOverlap
  (params (OtherActor :type Actor%20Object%20Reference))
  (Networking|SwitchHasAuthority
    (:Authority
      (bind _asdungeon_runners_character (Utilities|Casting|CastToDungeonRunnersCharacter OtherActor))
      (bind _returnvalue (Game|SpawnActorfromClass (Variables|Default|GetSelectedClass) (Math|Conversions|ToTransform(Vector) (Transformation|GetActorLocation (Variables|Default|GetTeleport))) "Undefined" 0 0))
      (Pawn|Possess (Pawn|GetController _asdungeon_runners_character) _returnvalue)
      (CallFunction|ClientCharacterSelect _asdungeon_runners_character))))

(event EventTick
  (params (DeltaSeconds :type Float%20%28single-precision%29)))

(fn ConstructionScript)